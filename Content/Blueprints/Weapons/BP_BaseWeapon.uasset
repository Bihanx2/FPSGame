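; Base weapon Blueprint that tracks magazine and backpack ammo, both filled to their maximums on BeginPlay.
; Fire only decrements the magazine and prints the count, with no ammo check or projectile logic.
; Reload sets the magazine to the lesser of capacity and backpack ammo, deducting that amount from the backpack and discarding leftover rounds.
; Query functions report whether the magazine has ammo or is full and whether the backpack has ammo.
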(event EventBeginPlay
  (Variables|Default|SetCurrentAmmoInMag (Variables|Default|GetMaxAmmoInMag))
  (Variables|Default|SetCurrentAmmoInBackpack (Variables|Default|GetMaxAmmoInBackpack)))

(fn ConstructionScript)

(fn Fire
  (bind _output_get (Variables|Default|SetCurrentAmmoInMag (- (Variables|Default|GetCurrentAmmoInMag) 1)))
  (Development|PrintString (Utilities|String|ToString(Integer) _output_get)))

(fn Reload
  (Variables|Default|SetCurrentAmmoInMag (Math|Integer|Min(Integer) (Variables|Default|GetMaxAmmoInMag) (Variables|Default|GetCurrentAmmoInBackpack)))
  (Variables|Default|SetCurrentAmmoInBackpack (- (Variables|Default|GetCurrentAmmoInBackpack) (Math|Integer|Min(Integer) (Variables|Default|GetMaxAmmoInMag) (Variables|Default|GetCurrentAmmoInBackpack)))))

(fn HaveAmmoinMag
  (return (> (Variables|Default|GetCurrentAmmoInMag) 0) (== (Variables|Default|GetCurrentAmmoInMag) (Variables|Default|GetMaxAmmoInMag))))

(fn HaveAmmoinBackpack
  (return (> (Variables|Default|GetCurrentAmmoInBackpack) 0)))