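; ImpactEffect is a weapon impact Blueprint that plays visual and audio feedback at a hit point when it begins play.
; It first builds a decal rotation from the HitResult normal with a random yaw.
; It then switches on the physical material's surface type, though only the default case is wired.
; That case spawns an emitter and sound, and attaches a limited-lifespan decal to the hit component and bone.
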(event EventBeginPlay
  (bind _hitresult (Variables|Default|GetHitResult))
  (bind _hitresult_2 (Variables|Default|GetHitResult))
  (bind _decal_size (Variables|Default|GetDecal%20Size))
  (bind _normal (Collision|BreakHitResult _hitresult))
  (bind (_bblockinghit _binitialoverlap _time _location _impactpoint _normal_2 _impactnormal _physmat _hitactor _hitcomponent _hitbonename) (Collision|BreakHitResult _hitresult_2))
  (bind _returnvalue (Math|Conversions|ToVector(Float) _decal_size))
  (bind _returnvalue_2 (Math|Conversions|RotationFromXVector _normal))
  (bind (_roll _pitch) (Math|Rotator|BreakRotator _returnvalue_2))
  (Utilities|FlowControl|Sequence
    (:then_0
      (Variables|Default|SetRandomDecalRotation (Math|Rotator|MakeRotator _roll _pitch (Math|Random|RandomFloatinRange -1.8e+02 1.8e+02))))
    (:then_1
      (switch Utilities|FlowControl|Switch|SwitchonEPhysicalSurface (Variables|/Script/Engine.PhysicalMaterial|GetSurfaceType _physmat)
        (:SurfaceType_Default
          (Effects|SpawnEmitteratLocation (Variables|Default|GetDefaul%20FX) _impactpoint)
          (Audio|PlaySoundatLocation (Variables|Default|GetDefault%20Sound) _impactpoint)
          (Class|GameplayStatics|SpawnDecalAttached (Variables|Default|GetDefault%20Decal%20Mat) (Math|Vector|MakeVector (.x _returnvalue) (.y _returnvalue) (.z _returnvalue)) _hitcomponent _hitbonename _impactpoint (Variables|Default|GetRandomDecalRotation) "SnapToTarget" (Variables|Default|GetDecal%20Life%20Span)))))))

(fn ConstructionScript)